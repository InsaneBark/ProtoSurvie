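; Master Blueprint for equipment items in the survival game, covering pickup, UI description and equip toggling.
; Interact adds the item info and amount to the player's action bar inventory, then destroys the actor.
; SendCalltoItem forwards the description to the main HUD when the requested class matches its own.
; EquipItem, for weapon tools only, equips the item class or reverts to fists if already equipped, passing matching weapon info to the player.
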(event EventBeginPlay)

(event Collision|EventActorBeginOverlap
  (params (OtherActor :type Actor%20Object%20Reference)))

(event EventTick
  (params (DeltaSeconds :type Float%20%28single-precision%29)))

(event EventInteract
  (params (PlayerRef :type BP%20Player%20Character%20Object%20Reference))
  ;[1 1 1] Add to inventory
  (Default|AddtoInventory (Variables|/Game/SurvivalGame/Core/Blueprints/Character/BP_PlayerCharacter.BP_PlayerCharacter_C|GetActionBarWidget PlayerRef) (Variables|Default|GetItemInfo) (Variables|Default|GetItemAmount))
  (Actor|DestroyActor))

(event EventSendCalltoItem
  (params (MainHUDWidget :type WBP%20Main%20HUD%20Object%20Reference) (Class :type Actor%20Class%20Reference))
  (CallFunction|SendDescriptiontoUI MainHUDWidget Class))

(event EventEquipItem
  (params (PlayerReft :type BP%20Player%20Character%20Object%20Reference) (ItemInfo :type S%20Item%20Info%20Structure))
  (bind (_name _icon _isstackable_ _description _itemclass _bcanbeuse _itemamount _itemscale _bisharvestables_ _bisaweapontool_) (Utilities|Struct|BreakS_ItemInfo ItemInfo))
  (if _bisaweapontool_
    (if (== (Variables|/Game/SurvivalGame/Core/Blueprints/Character/BP_PlayerCharacter.BP_PlayerCharacter_C|GetEquipementEquip PlayerReft) _itemclass)
      (Variables|/Game/SurvivalGame/Core/Blueprints/Character/BP_PlayerCharacter.BP_PlayerCharacter_C|SetEquipementEquip PlayerReft "/Game/SurvivalGame/Core/Blueprints/Items/Tools/BPC_Fist.BPC_Fist_C")
      (Default|GetWhatEquipementInfoinHand PlayerReft (Variables|Default|GetWeaponFistInfo))
      (else
        (Variables|/Game/SurvivalGame/Core/Blueprints/Character/BP_PlayerCharacter.BP_PlayerCharacter_C|SetEquipementEquip PlayerReft _itemclass)
        (Default|GetWhatEquipementInfoinHand PlayerReft (Variables|Default|GetWeaponInfo))))))

(fn ConstructionScript)

(fn SendDescriptiontoUI
  (params (MainHUDWidget :type Object%20Object%20Reference) (Class :type Object%20Class%20Reference))
  (if (== Class (Utilities|GetClass self))
    (Class|ICrossHairDescription|SendDesctoUI(Message) MainHUDWidget (Variables|Default|GetItemInfo) (Variables|Default|GetItemAmount))
    (return)))