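; Base food item for the survival game that the player picks up into the inventory and eats to restore hunger.
; On BeginPlay it caches the player character, and interacting adds the item to the action bar inventory and destroys the actor.
; Using it adds saturation to the player's Food, capped at the maximum, and pauses hunger for a set duration.
; It also sends its info and amount to the main HUD description when the requested class matches its own.
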(event EventUseItem
  (bind _as_bp_player_character (Variables|Default|GetAs%20BP%20Player%20Character))
  (bind _as_bp_player_character_2 (Variables|Default|GetAs%20BP%20Player%20Character))
  (bind _output_get (Variables|/Game/SurvivalGame/Core/Blueprints/Character/BP_PlayerCharacter.BP_PlayerCharacter_C|SetFood _as_bp_player_character_2 (+ (Variables|/Game/SurvivalGame/Core/Blueprints/Character/BP_PlayerCharacter.BP_PlayerCharacter_C|GetFood _as_bp_player_character_2) (Variables|Default|GetFoodSaturation))))
  (if (> _output_get (Variables|/Game/SurvivalGame/Core/Blueprints/Character/BP_PlayerCharacter.BP_PlayerCharacter_C|GetMaxFood _as_bp_player_character_2))
    (Variables|/Game/SurvivalGame/Core/Blueprints/Character/BP_PlayerCharacter.BP_PlayerCharacter_C|SetFood _as_bp_player_character (Variables|/Game/SurvivalGame/Core/Blueprints/Character/BP_PlayerCharacter.BP_PlayerCharacter_C|GetMaxFood _as_bp_player_character)))
  (Default|HungerPausewhenEat _as_bp_player_character (Variables|Default|GetHungerTimerPauseDuration)))

(event EventSendCalltoItem
  (params (MainHUDWidget :type WBP%20Main%20HUD%20Object%20Reference) (Class :type Actor%20Class%20Reference))
  ;[1 1 1] Send the info of the targeting Object to descriptionOverlay in Main HUD Blueprints
  (CallFunction|SendDescriptiontoUI MainHUDWidget Class))

(event EventBeginPlay
  (bind _asbp_player_character (Utilities|Casting|CastToBP_PlayerCharacter (Game|GetPlayerCharacter 0)))
  (Variables|Default|SetAs%20BP%20Player%20Character _asbp_player_character))

(event EventInteract
  (params (PlayerRef :type BP%20Player%20Character%20Object%20Reference))
  ;[1 1 1] Add to inventory if the player interact with
  (Default|AddtoInventory (Variables|/Game/SurvivalGame/Core/Blueprints/Character/BP_PlayerCharacter.BP_PlayerCharacter_C|GetActionBarWidget (Variables|Default|GetAs%20BP%20Player%20Character)) (Variables|Default|GetItemInfo) (Variables|Default|GetItemAmount))
  (Actor|DestroyActor))

(fn ConstructionScript)

(fn SendDescriptiontoUI
  (params (MainHUDWidgetRef :type Object%20Object%20Reference) (ItemClass :type Object%20Class%20Reference))
  (if (== ItemClass (Utilities|GetClass self))
    (Class|ICrossHairDescription|SendDesctoUI(Message) MainHUDWidgetRef (Variables|Default|GetItemInfo) (Variables|Default|GetItemAmount))
    (return)))