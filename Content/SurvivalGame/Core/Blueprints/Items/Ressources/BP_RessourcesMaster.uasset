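; BP_RessourcesMaster is the master actor for resource pickups in the survival game.
; Interact adds its ItemInfo and ItemAmount to the player's action bar inventory, then destroys the actor.
; SendCalltoItem passes the item's info and amount to the main HUD description overlay when the given class matches its own.
; UseItem only prints that the item cannot be used.
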(event EventUseItem
  (Development|PrintString "Cant use This Item"))

(event EventSendCalltoItem
  (params (MainHUDWidget :type WBP%20Main%20HUD%20Object%20Reference) (Class :type Actor%20Class%20Reference))
  ;[1 1 1] Send the info of the targeting Object to descriptionOverlay in Main HUD Blueprints
  (CallFunction|SendDescriptiontoUI MainHUDWidget Class))

(event EventInteract
  (params (PlayerRef :type BP%20Player%20Character%20Object%20Reference))
  ;[1 1 1] Add to inventory if the player interact with
  (Default|AddtoInventory (Variables|/Game/SurvivalGame/Core/Blueprints/Character/BP_PlayerCharacter.BP_PlayerCharacter_C|GetActionBarWidget PlayerRef) (Variables|Default|GetItemInfo) (Variables|Default|GetItemAmount))
  (Actor|DestroyActor))

(fn ConstructionScript)

(fn SendDescriptiontoUI
  (params (MainHUDWidgetRef :type Object%20Object%20Reference) (ItemClass :type Object%20Class%20Reference))
  (if (== ItemClass (Utilities|GetClass self))
    (Class|ICrossHairDescription|SendDesctoUI(Message) MainHUDWidgetRef (Variables|Default|GetItemInfo) (Variables|Default|GetItemAmount))
    (return)))