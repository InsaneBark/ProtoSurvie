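; Harvestable logs item for the survival game that the player picks up by interacting with it.
; Interact adds one unit of its ItemInfo to the player's inventory through the ActionBarWidget, then destroys the actor.
; Tick prints CurrentHP and FixeSpawnWhenDestroy every frame as debug output, with no damage or spawn logic in this graph.
; The construction script only calls the parent.
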(event EventBeginPlay
  (|CallParentFunction) ; This node is disabled and will not be called.\nDrag off pins to build functionality.
)

(event Collision|EventActorBeginOverlap
  (params (OtherActor :type Actor%20Object%20Reference))
  (|CallParentFunction OtherActor) ; This node is disabled and will not be called.\nDrag off pins to build functionality.
)

(event EventTick
  (params (DeltaSeconds :type Float%20%28single-precision%29))
  (Development|PrintString (Utilities|String|ToString(Float) (Variables|Default|GetCurrentHP)))
  (Development|PrintString (Utilities|String|ToString(Integer) (Variables|Default|GetFixeSpawnWhenDestroy))))

(event EventInteract
  (params (PlayerRef :type BP%20Player%20Character%20Object%20Reference))
  (Default|AddtoInventory (Variables|/Game/SurvivalGame/Core/Blueprints/Character/BP_PlayerCharacter.BP_PlayerCharacter_C|GetActionBarWidget PlayerRef) (Variables|Default|GetItemInfo) 1)
  (Actor|DestroyActor))

(fn ConstructionScript
  (|CallParentFunction))