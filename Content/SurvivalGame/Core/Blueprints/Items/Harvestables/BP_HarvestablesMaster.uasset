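; Base actor for harvestable items in the survival game, which take tool damage, drop resources and can offer a collectable.
; Damage applies only when the tool tier meets the item tier; at zero HP, spawn loops create drops and destroy the actor.
; Collecting swaps the mesh, clears the collectable flag and adds a random amount to the player's action bar.
; It also sends its item description to the main HUD when targeted.
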(event Custom|ActorDestroy
  ;[1 1 1] DestroyActor and spawnRessources
  (if (Variables|Bools|GetbIsCollectables?) ; Check if It Collectable when destroy
    (CallFunction|SpawnRessourcesandCollectables)
    (else
      (CallFunction|SpawnRessources))))

(event EventBeginPlay
  (Variables|Hp|SetCurrentHP (Variables|Hp|GetMaxHP)))

(event EventIsCollectables
  (params (PlayerCharacter :type BP%20Player%20Character%20Object%20Reference))
  ;[1 1 1] CollectablesItems
  (CallFunction|AdditemtoInventoryifIsCollectables PlayerCharacter))

(event Collision|EventActorBeginOverlap
  (params (OtherActor :type Actor%20Object%20Reference)))

(event EventSendCalltoItem
  (params (MainHUDWidget :type WBP%20Main%20HUD%20Object%20Reference) (Class :type Actor%20Class%20Reference))
  ;[1 1 1] Send the info of the targeting Object to descriptionOverlay in Main HUD Blueprints
  (UIrelated|SendDescriptiontoUI MainHUDWidget Class))

(event EventIsHarvestables
  (params (DamageInput :type Float%20%28single-precision%29) (ToolTier :type Integer))
  ;[1 1 1] Damage Actor with damage Input and check if destroy
  (DamageActor|DamagesItemandDestroyCommand DamageInput ToolTier))

(fn ConstructionScript)

(fn SendDescriptiontoUI
  (params (MainHUDWidget :type Object%20Object%20Reference) (ItemClass :type Object%20Class%20Reference))
  (if (== ItemClass (Utilities|GetClass self))
    (Class|ICrossHairDescription|SendDesctoUI(Message) MainHUDWidget (Variables|ItemInfo|GetItemInfo))
    (return)))

(fn DamagesItemandDestroyCommand
  (params (DamageInput :type Float%20%28single-precision%29) (ToolTier :type Integer))
  (if (>= ToolTier (Variables|ItemTier|GetItemTier))
    (bind _output_get (Variables|Hp|SetCurrentHP (- (Variables|Hp|GetCurrentHP) DamageInput)))
    (if (<= _output_get 0.0)
      (Variables|Hp|SetCurrentHP 0.0)
      (CallFunction|ActorDestroy)
      (return))))

(fn AdditemtoInventoryifIsCollectables
  (params (self2 :type BP%20Player%20Character%20Object%20Reference))
  (if (Variables|Bools|GetbIsCollectables?)
    (Variables|Bools|SetbIsCollectables? false)
    (Components|StaticMesh|SetStaticMesh (Variables|Default|GetMesh) (Variables|ItemCollected|Mesh|GetMeshToBeReplace))
    (bind _output_get (Variables|ItemCollected|SetAmountToAddWhenCollected (Math|Random|RandomInteger 6)))
    (if (< _output_get 3)
      (bind _output_get_2 (Variables|ItemCollected|SetAmountToAddWhenCollected 3)))
    (Default|AddtoInventory (Variables|/Game/SurvivalGame/Core/Blueprints/Character/BP_PlayerCharacter.BP_PlayerCharacter_C|GetActionBarWidget self2) (Variables|ItemInfo|GetItemInfoToAdd) _output_get_2)))

(fn SpawnRessourcesandCollectables
  (Utilities|FlowControl|Sequence
    (:then_0
      (for _index (range 0 (Math|Random|RandomInteger (Variables|WhenDestroy|Spawn|GetMaxSpawnWhenDestroy)))
        (Game|SpawnActorfromClass (Variables|WhenDestroy|Class|GetItemClassToSpawnWhenDestroy) (Math|Transform|MakeTransform (Transformation|GetActorLocation) "0, 0, 0" (Variables|WhenDestroy|Scale|GetActorScaleToSpawnWhenDestroy)) "Undefined" 0 0)
        (Actor|DestroyActor)))
    (:then_1
      (for _index_2 (range 0 (Math|Random|RandomInteger (Variables|WhenDestroy|Spawn|GetMaxSpawnWhenDestroyWithCollectables)))
        (Game|SpawnActorfromClass (Variables|WhenDestroy|Class|GetItemClassToSplawnWhenDestroyCollectable) (Math|Transform|MakeTransform (+ (Transformation|GetActorLocation) "0,25.000000, 0") "0, 0, 0" (Variables|WhenDestroy|Scale|GetActorScaleToSpawnWhenDestroyCollectables)) "Undefined" 0 0)
        (Actor|DestroyActor)))))

(fn SpawnRessources
  (if (Variables|Bools|GetbIsSpawnNumberRandom?)
    (for _index (range 0 (Math|Random|RandomInteger (Variables|WhenDestroy|Spawn|GetMaxSpawnWhenDestroy)))
      (Game|SpawnActorfromClass (Variables|WhenDestroy|Class|GetItemClassToSpawnWhenDestroy) (Math|Transform|MakeTransform (Transformation|GetActorLocation) "0, 0, 0" (Variables|WhenDestroy|Scale|GetActorScaleToSpawnWhenDestroy)) "Undefined" 0 0)
      (Actor|DestroyActor)
      (return))
    (else
      (for _index_2 (range 0 (Variables|WhenDestroy|Spawn|GetFixeSpawnWhenDestroy))
        (Game|SpawnActorfromClass (Variables|WhenDestroy|Class|GetItemClassToSpawnWhenDestroy) (Math|Transform|MakeTransform (Transformation|GetActorLocation) "0, 0, 0" (Variables|WhenDestroy|Scale|GetActorScaleToSpawnWhenDestroy)) "Undefined" 0 0)
        (Actor|DestroyActor)
        (return)))))