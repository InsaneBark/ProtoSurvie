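; StaminaPotion is a pickup item that spins in the world and goes into the player's inventory when interacted with.
; Interact passes its ItemInfo to the player character's InventoryWidget with an amount of zero, calling DestroyActor both before and after.
; UseItem is a placeholder that only prints a debug string, with no stamina effect.
; Tick yaws the root by delta time plus one degree, so spin speed depends on frame rate.
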(event EventTick
  (params (DeltaSeconds :type Float%20%28single-precision%29))
  (Transformation|AddLocalRotation (Variables|Default|GetDefaultSceneRoot) (Math|Rotator|MakeRotator 0.0 0.0 (+ DeltaSeconds 1.0)) false false))

(event EventInteract
  (params (PlayerRef :type BP%20Player%20Character%20Object%20Reference))
  (Actor|DestroyActor)
  (bind _asbp_player_character (Utilities|Casting|CastToBP_PlayerCharacter (Game|GetPlayerCharacter 0)))
  (Default|AddtoInventory (Variables|/Game/SurvivalGame/Core/Blueprints/Character/BP_PlayerCharacter.BP_PlayerCharacter_C|GetInventoryWidget _asbp_player_character) (Variables|Default|GetItemInfo))
  (Actor|DestroyActor))

(event EventUseItem
  (Development|PrintString "UseStamina"))

(fn ConstructionScript
  (|CallParentFunction))